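; BP_E_Oso is a bear enemy that wanders around the location where it spawns.
; On BeginPlay it stores that origin, then line-traces downward between independently randomized XY points within RadioOso, with debug drawing, from a fixed world height.
; AI MoveTo sends it to the impact point.
; On success it waits briefly and picks another point; a failed move has no retry, so wandering stops.
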(event `self.ReceiveBeginPlay`
  (bind (_ubicacion_i_oso_x _ubicacion_i_oso_y) (`KismetMathLibrary.BreakVector` (`self.Ubicacion_I_Oso`)))
  (bind _returnvalue (+ (`KismetMathLibrary.RandomFloatInRange` (* (`self.Radio_Oso`) -1.0) (`self.Radio_Oso`)) _ubicacion_i_oso_y))
  (bind _returnvalue_2 (+ (`KismetMathLibrary.RandomFloatInRange` (* (`self.Radio_Oso`) -1.0) (`self.Radio_Oso`)) _ubicacion_i_oso_x))
  (set `self.Ubicacion_I_Oso` (`self.K2_GetActorLocation`))
  (bind _outhit (`KismetSystemLibrary.LineTraceSingle` :`Start` (`KismetMathLibrary.MakeVector` _returnvalue_2 _returnvalue 2.0) :`End` (`KismetMathLibrary.MakeVector` _returnvalue_2 _returnvalue -20000.0) :`TraceChannel` "TraceTypeQuery1" :`DrawDebugType` "ForDuration" :`DrawTime` 100.0 :!label _label))
  (`|AIMoveTo` self (`.ImpactPoint` (`GameplayStatics.BreakHitResult` _outhit)) null
    (:`OnSuccess`
      (`KismetSystemLibrary.Delay` 2.0)
      (goto _label))))

(fn `UserConstructionScript`)