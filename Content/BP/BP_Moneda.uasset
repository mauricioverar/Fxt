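; BP_Moneda is a coin pickup that the player character collects by touching it.
; On BeginPlay it caches the Gi_Juego game instance, which holds the Monedas coin count.
; When its Box overlaps a BP_Personaje, it increments that count, destroys itself and plays the Camera_Shutter sound at its location.
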(event `self.ReceiveBeginPlay`
  (bind _asgi_juego (cast `/Game/BP/Gi_Juego` (`GameplayStatics.GetGameInstance`)))
  (set `self.As Gi Juego` _asgi_juego))

(event `self.Box.OnComponentBeginOverlap`
  (params (OverlappedComponent :type "PrimitiveComponent Object Reference") (OtherActor :type "Actor Object Reference") (OtherComp :type "PrimitiveComponent Object Reference") (OtherBodyIndex :type Integer) (bFromSweep :type Boolean) (SweepResult :type "HitResult Structure (by ref)"))
  (cast `/Game/Personaje/BP_Personaje` OtherActor)
  (set `/Game/BP/Gi_Juego.Monedas` (+ (`/Game/BP/Gi_Juego.Monedas` (`self.As Gi Juego`)) 1) (`self.As Gi Juego`))
  (`self.K2_DestroyActor`)
  (`GameplayStatics.PlaySoundAtLocation` "/Engine/VREditor/Sounds/UI/Camera_Shutter.Camera_Shutter" (`self.K2_GetActorLocation`) (struct) 1.0 1.0 0.0 null null null))

(fn `UserConstructionScript`)